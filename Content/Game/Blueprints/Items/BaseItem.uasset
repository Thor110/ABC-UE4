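; BaseItem is a pickup item actor that adds itself to the player's HUD inventory and can restore health and stamina when used.
; Its construction script fills the item info struct and sets the mesh; BeginPlay creates the pickup prompt widget, which draw and destroy events toggle alongside an overlap flag.
; A handler bound to the character's pickup dispatcher stores the struct, refreshes the inventory and destroys the actor, if overlapping with collision enabled.
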(event Custom|DrawPickupText
  ;[1 1 1] Overlapping Item
  (UserInterface|Viewport|AddtoViewport (Variables|Default|GetPickupTextReference) 0)
  (Variables|Default|SetOverlapping true))

(event Custom|DestroyPickupText
  ;[1 1 1] Overlapping Item
  (Widget|RemovefromParent (Variables|Default|GetPickupTextReference))
  (Variables|Default|SetOverlapping false))

(event Custom|PickupItem_Event_0
  (bind _characterreference (Variables|Default|GetCharacterReference))
  (bind _mycharacterhudreference (Variables|/Game/Game/Blueprints/Player/MyCharacter.MyCharacter_C|GetMyCharacterHUDReference _characterreference))
  ;[1 1 1] Pickup Item
  (if (and (Collision|GetActorEnableCollision) (Variables|Default|GetOverlapping))
    (Utilities|Array|Add (Variables|/Game/Game/Blueprints/Player/MyCharacterHUD.MyCharacterHUD_C|GetInventory _mycharacterhudreference) (Variables|Default|GetItemInfo))
    (Widget|RemovefromParent (Variables|Default|GetPickupTextReference))
    (Default|RefreshInventory _mycharacterhudreference)
    (Actor|DestroyActor)))

(event EventBeginPlay
  (bind _iteminfo (Variables|Default|GetItemInfo))
  (bind (_item _icon _pickuptext) (Utilities|Struct|BreakInventoryStructure _iteminfo))
  ;[1 1 1] Draw Pickup Text
  (bind _returnvalue (UserInterface|CreateWidget "/Game/Game/Blueprints/Player/PickupText.PickupText_C" (Game|GetPlayerController 0)))
  (Variables|Default|SetPickupTextReference _returnvalue)
  (Utilities|Struct|SetmembersinInventoryStructure _iteminfo self)
  (Variables|/Game/Game/Blueprints/Player/PickupText.PickupText_C|SetPickupActor (Variables|Default|GetPickupTextReference) _item)
  (Variables|/Game/Game/Blueprints/Player/PickupText.PickupText_C|SetPickupText (Variables|Default|GetPickupTextReference) _pickuptext)
  (bind _asmy_character (Utilities|Casting|CastToMyCharacter (Game|GetPlayerCharacter 0)))
  (bind _output_get (Variables|Default|SetCharacterReference _asmy_character))
  (EventDispatchers|AssignPickupItem _output_get (delegate Custom|PickupItem_Event_0)))

(event EventUseAction
  (bind _characterreference (Variables|Default|GetCharacterReference))
  ;[1 1 1] Use Item
  (Variables|/Game/Game/Blueprints/Player/MyCharacter.MyCharacter_C|SetHealth _characterreference (+ (Variables|/Game/Game/Blueprints/Player/MyCharacter.MyCharacter_C|GetHealth _characterreference) (Variables|Default|GetAddHealth)))
  (Variables|/Game/Game/Blueprints/Player/MyCharacter.MyCharacter_C|SetStamina _characterreference (+ (Variables|/Game/Game/Blueprints/Player/MyCharacter.MyCharacter_C|GetStamina _characterreference) (Variables|Default|GetAddStamina)))
  (Actor|DestroyActor))

(fn ConstructionScript
  (Utilities|Struct|SetmembersinInventoryStructure (Variables|Default|GetItemInfo) self (Variables|Default|GetItemIcon) (Variables|Default|GetItemPickupText) (Variables|Default|GetItemActionText))
  (Components|StaticMesh|SetStaticMesh (Variables|Default|GetStaticMesh) (Variables|Default|GetItemStaticMesh)))