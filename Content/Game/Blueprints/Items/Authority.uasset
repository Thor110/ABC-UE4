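; Item actor that displays whether the running instance has network authority, as a "Server" or "Client" text label.
; On BeginPlay, Switch Has Authority sets the label and mesh material for each role, and also recolors the text on remote instances.
; Each Tick, the text takes the rotation of player 0's MyCharacter with yaw turned 180 degrees, so it faces opposite that character's heading.
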(event EventBeginPlay
  (bind _textrender (Variables|Default|GetTextRender))
  (bind _staticmesh (Variables|Default|GetStaticMesh))
  (Networking|SwitchHasAuthority
    (:Authority
      (bind _output_get (Variables|Default|SetServerOrClient "Server"))
      (Rendering|Components|TextRender|SetText _textrender _output_get)
      (Rendering|Material|SetMaterial _staticmesh 0 0))
    (:Remote
      (bind _output_get_2 (Variables|Default|SetServerOrClient "Client"))
      (Rendering|Components|TextRender|SetText _textrender _output_get_2)
      (Rendering|Material|SetMaterial _staticmesh 0 0)
      (Rendering|Components|TextRender|SetTextRenderColor _textrender (Math|Color|MakeColor 255 0 0 0)))))

(event EventTick
  (params (DeltaSeconds :type Float%20%28single-precision%29))
  (bind _asmy_character (Utilities|Casting|CastToMyCharacter (Game|GetPlayerCharacter 0)))
  (Transformation|SetWorldRotation (Variables|Default|GetTextRender) (Math|Rotator|MakeRotator (.Roll (Math|Rotator|BreakRotator (Transformation|GetActorRotation _asmy_character))) (.Pitch (Math|Rotator|BreakRotator (Transformation|GetActorRotation _asmy_character))) (- (.Yaw (Math|Rotator|BreakRotator (Transformation|GetActorRotation _asmy_character))) 1.8e+02)) false false))

(fn ConstructionScript)