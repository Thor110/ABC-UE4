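; Game instance that manages multiplayer sessions for lobby hosting, joining, restarting and leaving.
; Hosting creates a session using the player count and LAN settings, sets state flags and opens the level as a listen server.
; Joining takes a server-list result, while closing destroys the session and either returns to MainMenu or quits the game.
; Restart destroys and recreates the session, then reopens the current level as a listen server.
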(event Custom|DestroyLobby
  (params (InController :type Player%20Controller%20Object%20Reference))
  ;[1 1 1] Host Quit Game
  (|DestroySession InController
    (:OnSuccess
      (Variables|Default|SetInGame false)
      (Variables|Default|SetIsOnline false)
      (Development|ExecuteConsoleCommand "quit" 0))
    (:OnFailure
      (Development|PrintString "Destroy Session Failed!"))))

(event Custom|JoinFromServerList
  (params (Server :type Blueprint%20Session%20Result%20Structure))
  ;[1 1 1] Join From Server List
  (|JoinSession (Game|GetPlayerController 0) Server
    (:OnSuccess
      (Variables|Default|SetIsOnline true)
      (Variables|Default|SetInGame true)
      (Development|PrintString "CREATE CHARACTER WIDGET")
      ;[1 1 1] Enable Mouse Cursor
      (Variables|/Script/Engine.PlayerController|SetbShowMouseCursor (Game|GetPlayerController 0) false))
    (:OnFailure
      (Development|PrintString "Failed To Join Server"))))

(event Custom|RestartSession
  (params (PlayerController :type Player%20Controller%20Object%20Reference))
  ;[1 1 1] Restart Session
  (|DestroySession PlayerController
    (:then
      (Development|PrintString "Closing Session"))
    (:OnSuccess
      (|Session PlayerController (Variables|Default|GetNumberPlayers) (Variables|Default|GetEnable%20LAN)
        (:then
          (Development|PrintString "Recreationg Session"))
        (:OnSuccess
          (bind _returnvalue (Game|GetCurrentLevelName true))
          (Game|OpenLevel(byName) (Utilities|String|StringToName _returnvalue) true "listen"))
        (:OnFailure
          (Development|PrintString "Failed To Recreate Session Kicked Out"))))
    (:OnFailure
      (Development|PrintString "Failed To Destroy Session"))))

(event Custom|ServerCloseLobby
  (params (InController :type Player%20Controller%20Object%20Reference))
  ;[1 1 1] Host Quit To Main Menu Or Quit Match
  (|DestroySession InController
    (:OnSuccess
      (Variables|Default|SetInGame false)
      (Variables|Default|SetIsOnline false)
      (Game|OpenLevel(byName) "MainMenu"))
    (:OnFailure
      ;[1 1 1] Host Quit Game
      (Development|PrintString "Destroy Session Failed!"))))

(event Custom|SpawnPlayer)

(event Custom|ServerHostLobby
  (params (InController :type Player%20Controller%20Object%20Reference) (LevelName :type Name))
  ;[1 1 1] Host Lobby
  (|Session InController (Variables|Default|GetNumberPlayers) (Variables|Default|GetEnable%20LAN)
    (:OnSuccess
      (Variables|Default|SetIsHost true)
      (Variables|Default|SetLobbyCameraActive true)
      (Variables|Default|SetInGame true)
      (Variables|Default|SetIsOnline true)
      (Development|PrintString "HOSTED")
      (Game|OpenLevel(byName) LevelName true "listen")
      ;[1 1 1] Enable Mouse Cursor
      (Variables|/Script/Engine.PlayerController|SetbShowMouseCursor (Game|GetPlayerController 0) false))
    (:OnFailure
      (Development|PrintString "Create Session Failed!" true true "(R=0.880000,G=0.006366,B=0.000000,A=1.000000)"))))