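; MyHUD is a HUD Blueprint that draws a crosshair at the center of the screen.
; On each HUD draw it stores the screen size, then draws the Crosshair texture scaled down and offset to center it, only while ShowCrossHair is true.
; The drawing uses the canvas-based DrawTextureSimple call rather than a UMG widget, and the construction script is empty.
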(event EventDrawHUD
  (params (SizeX :type Integer) (SizeY :type Integer))
  ;[1 1 1] Draw Crosshair
  (Variables|TestVariables|SetSizeX SizeX)
  (Variables|TestVariables|SetSizeY SizeY)
  (if (Variables|InventoryVariables|GetShowCrossHair)
    (Class|HUD|DrawTextureSimple "/Game/Game/Assets/Textures/GUI/crosshair.crosshair" (- (Math|Conversions|ToFloat(Integer) (/ SizeX 2)) 16.0) (- (Math|Conversions|ToFloat(Integer) (/ SizeY 2)) 16.0) 0.125 false)))

(fn ConstructionScript)